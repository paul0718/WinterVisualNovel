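; BP_Door_01 is a double corridor door for the Japanese school, built to swing away from or toward the player's side, but currently inert.
; BeginPlay stores both leaves' world yaw, and the trigger box's overlap events are empty.
; An unconnected chain tests which side the player stands on, then uses a timeline to rotate the leaves in mirrored directions and activate a box on finish.
; Nothing triggers that chain.
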(event OnComponentBeginOverlap(Box_T)
  (params (OverlappedComponent :type Primitive%20Component%20Object%20Reference) (OtherActor :type Actor%20Object%20Reference) (OtherComp :type Primitive%20Component%20Object%20Reference) (OtherBodyIndex :type Integer) (bFromSweep :type Boolean) (SweepResult :type Hit%20Result%20Structure%20%28by%20ref%29)))

(event OnComponentEndOverlap(Box_T)
  (params (OverlappedComponent :type Primitive%20Component%20Object%20Reference) (OtherActor :type Actor%20Object%20Reference) (OtherComp :type Primitive%20Component%20Object%20Reference) (OtherBodyIndex :type Integer)))

(event EventBeginPlay
  (Variables|Default|SetReturn%20Value%20Z%20%28Yaw%29_0 (.yaw (Transformation|GetWorldRotation (Variables|Default|GetSM_Corridor_Door_02))))
  (Variables|Default|SetReturn%20Value%20Z%20%28Yaw%29 (.yaw (Transformation|GetWorldRotation (Variables|Default|GetSM_Corridor_Door_01)))))

(fn ConstructionScript)