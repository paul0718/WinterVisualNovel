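; BP_Door_04 is a double corridor door that swings open automatically when something overlaps its trigger box, provided it is Openable.
; On overlap, the player pawn's local-space side of the door picks the swing direction, and timeline T rotates both leaves in opposite yaw to 85 degrees.
; Ending the overlap reverses the timeline to close them.
; The yaws cached at BeginPlay are not used in the rotation.
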(event OnComponentBeginOverlap(Box_T)
  (params (OverlappedComponent :type Primitive%20Component%20Object%20Reference) (OtherActor :type Actor%20Object%20Reference) (OtherComp :type Primitive%20Component%20Object%20Reference) (OtherBodyIndex :type Integer) (bFromSweep :type Boolean) (SweepResult :type Hit%20Result%20Structure%20%28by%20ref%29))
  (if (Variables|Default|GetOpenable)
    (Variables|Default|SetTB (> (.y (Math|Vector|UnrotateVector (- (Transformation|GetActorLocation) (Transformation|GetActorLocation (Game|Player|GetPlayerPawn 0))) (Transformation|GetActorRotation))) 0.0))
    (bind _y (Timeline|T Play)
      (:Update
        (Transformation|SetRelativeRotation (Variables|Default|GetSM_Corridor_Door_01) (Math|Rotator|MakeRotator 0.0 0.0 (* _y (Math|Float|SelectFloat 85.0 -85.0 (Variables|Default|GetTB)))) false false)
        (Transformation|SetRelativeRotation (Variables|Default|GetSM_Corridor_Door_02) (Math|Rotator|MakeRotator 0.0 0.0 (* (* _y (Math|Float|SelectFloat 85.0 -85.0 (Variables|Default|GetTB))) -1.0)) false false))
      (:Finished
        (Components|Activation|Activate (Variables|Default|GetBox_T) true)))))

(event OnComponentEndOverlap(Box_T)
  (params (OverlappedComponent :type Primitive%20Component%20Object%20Reference) (OtherActor :type Actor%20Object%20Reference) (OtherComp :type Primitive%20Component%20Object%20Reference) (OtherBodyIndex :type Integer))
  (if (Variables|Default|GetOpenable)
    (bind _y (Timeline|T Reverse)
      (:Update
        (Transformation|SetRelativeRotation (Variables|Default|GetSM_Corridor_Door_01) (Math|Rotator|MakeRotator 0.0 0.0 (* _y (Math|Float|SelectFloat 85.0 -85.0 (Variables|Default|GetTB)))) false false)
        (Transformation|SetRelativeRotation (Variables|Default|GetSM_Corridor_Door_02) (Math|Rotator|MakeRotator 0.0 0.0 (* (* _y (Math|Float|SelectFloat 85.0 -85.0 (Variables|Default|GetTB))) -1.0)) false false))
      (:Finished
        (Components|Activation|Activate (Variables|Default|GetBox_T) true)))))

(event EventBeginPlay
  (Variables|Default|SetReturn%20Value%20Z%20%28Yaw%29_0 (.yaw (Transformation|GetWorldRotation (Variables|Default|GetSM_Corridor_Door_02))))
  (Variables|Default|SetReturn%20Value%20Z%20%28Yaw%29 (.yaw (Transformation|GetWorldRotation (Variables|Default|GetSM_Corridor_Door_01)))))

(fn ConstructionScript)