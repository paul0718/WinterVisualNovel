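; Automatic toilet door actor that slides open when something overlaps its trigger box and closes when the overlap ends.
; A timeline drives the door mesh's relative X location, playing on overlap begin and reversing on overlap end.
; Lock sets a flag and forces the door closed, while Unlock only clears the flag.
; Either that flag or PermaLock makes the trigger ignore overlaps in both directions.
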(event OnComponentBeginOverlap(Box_T)
  (params (OverlappedComponent :type Primitive%20Component%20Object%20Reference) (OtherActor :type Actor%20Object%20Reference) (OtherComp :type Primitive%20Component%20Object%20Reference) (OtherBodyIndex :type Integer) (bFromSweep :type Boolean) (SweepResult :type Hit%20Result%20Structure%20%28by%20ref%29))
  (if (not (Variables|Default|GetPermaLock))
    (if (not (Variables|Default|GetIsLocked))
      (bind _y (Timeline|T Play)
        (:Update
          (Transformation|SetRelativeTransform (Variables|Default|GetSM_Toilet_Door_01) (Math|Transform|MakeTransform (Math|Vector|MakeVector (* _y -9e+01) 0.0 0.0) "0, 0, 0" "1.000000,1.000000,1.000000") false false))))))

(event OnComponentEndOverlap(Box_T)
  (params (OverlappedComponent :type Primitive%20Component%20Object%20Reference) (OtherActor :type Actor%20Object%20Reference) (OtherComp :type Primitive%20Component%20Object%20Reference) (OtherBodyIndex :type Integer))
  (if (not (Variables|Default|GetPermaLock))
    (if (not (Variables|Default|GetIsLocked))
      (bind _y (Timeline|T Reverse)
        (:Update
          (Transformation|SetRelativeTransform (Variables|Default|GetSM_Toilet_Door_01) (Math|Transform|MakeTransform (Math|Vector|MakeVector (* _y -9e+01) 0.0 0.0) "0, 0, 0" "1.000000,1.000000,1.000000") false false))))))

(event Custom|ForceClose
  (bind _y (Timeline|T Reverse)
    (:Update
      (Transformation|SetRelativeTransform (Variables|Default|GetSM_Toilet_Door_01) (Math|Transform|MakeTransform (Math|Vector|MakeVector (* _y -9e+01) 0.0 0.0) "0, 0, 0" "1.000000,1.000000,1.000000") false false))))

(event EventLock
  (Variables|Default|SetIsLocked true)
  (CallFunction|ForceClose))

(event EventUnlock
  (Variables|Default|SetIsLocked false))

(fn ConstructionScript)