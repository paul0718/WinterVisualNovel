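; BP_ItemInteractBox is an overlap-triggered interactable that starts a side-plot dialogue when the player interacts with it.
; On begin and end overlap with a BP_PlayerCharacter, it registers or clears itself as the current interactable through the character's ACPlayer.
; Its Interact event spawns an actor of the SidePlot class and passes it to the interacting player's EnterDialogueMode.
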(event EventBeginPlay)

(event Collision|EventActorBeginOverlap
  (params (OtherActor :type Actor%20Object%20Reference))
  (bind _asbp_player_character (Utilities|Casting|CastToBP_PlayerCharacter OtherActor))
  (Default|SetCurrentInteractable (Variables|/Game/Blueprint/PlayerControl/BP_PlayerCharacter.BP_PlayerCharacter_C|GetAC_Player _asbp_player_character) self))

(event EventTick
  (params (DeltaSeconds :type Float%20%28single-precision%29)))

(event Collision|EventActorEndOverlap
  (params (OtherActor :type Actor%20Object%20Reference))
  (bind _asbp_player_character (Utilities|Casting|CastToBP_PlayerCharacter OtherActor))
  (Default|LeaveInteractable (Variables|/Game/Blueprint/PlayerControl/BP_PlayerCharacter.BP_PlayerCharacter_C|GetAC_Player _asbp_player_character) self))

(event EventInteract
  (params (From%20Player :type AC%20Player%20Object%20Reference))
  (bind _returnvalue (Game|SpawnActorfromClass (Variables|Default|GetSidePlot) (Math|Transform|MakeTransform "0, 0, 0" "0, 0, 0" "1.000000,1.000000,1.000000") "Undefined" "MultiplyWithRoot" 0 0))
  (Default|EnterDialogueMode From%20Player _returnvalue))

(fn ConstructionScript)