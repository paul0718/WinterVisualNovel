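; Debug actor component for the player character that provides a key shortcut to skip plot progress.
; On BeginPlay it casts its owner to BP_PlayerCharacter and caches that character's ACPlayer component.
; Pressing the debug key U increments the plot manager's EventMarker twice, then spawns a BI_18_Night actor and immediately sends it an interact message with the player reference.
; Tick is unused.
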(event EventBeginPlay
  (bind _asbp_player_character (Utilities|Casting|CastToBP_PlayerCharacter (Components|GetOwner)))
  (Variables|Default|SetPlayerReference (Variables|/Game/Blueprint/PlayerControl/BP_PlayerCharacter.BP_PlayerCharacter_C|GetAC_Player _asbp_player_character)))

(event EventTick
  (params (DeltaSeconds :type Float%20%28single-precision%29)))

(event Input|KeyboardEvents|DebugKeyY
  (params (Key :type Key%20Structure :default "None") (ActionValue :type Input%20Action%20Value%20Structure)))

(event Input|KeyboardEvents|DebugKeyU
  (params (Key :type Key%20Structure :default "None") (ActionValue :type Input%20Action%20Value%20Structure))
  (bind _playerreference (Variables|Default|GetPlayerReference))
  (bind _plotmanagerref (Variables|/Game/Blueprint/AC_Player.AC_Player_C|GetPlotManagerRef _playerreference))
  (bind _eventmarker (Variables|/Game/Blueprint/BP_PlotManager.BP_PlotManager_C|GetEventMarker _plotmanagerref))
  (:Pressed
    (Math|Integer|IncrementInt _eventmarker
      (:%20%20
        (Math|Integer|IncrementInt _eventmarker
          (:%20%20
            (bind _returnvalue (Game|SpawnActorfromClass "/Game/Blueprint/Interactables/BI_1-8_Night.BI_1-8_Night_C" (Math|Transform|MakeTransform "0, 0, 0" "0, 0, 0" "1.000000,1.000000,1.000000") "Undefined" "MultiplyWithRoot" 0 0))
            (Class|BPIInteraction|Interact(Message) _returnvalue _playerreference)))))))