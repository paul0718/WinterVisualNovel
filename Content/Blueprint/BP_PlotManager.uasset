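; Manages story flow, opening the game with the Ch10 dialogue cutscene and pre-spawning Ichinose's plot actors.
; Chapter tags drive freeroam: interactables are shown or hidden, doors toggle lock messages, and Ichinose's interact boxes receive the plot matching current progress.
; An event-marker check launches the Ch13 cutscene once every "1-2" interact box's plot is viewed.
; It also shows a one-time tutorial widget with the mouse cursor.
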(event Custom|Hide%20All%20Interactable
  (bind _outactors (Actor|GetAllActorswithTag "Chapter"))
  (for _array_element _outactors
    (if (Actor|ActorHasTag _array_element "Door")
      (Class|BPIDoor|Unlock(Message) _array_element)
      (else
        (Rendering|SetActorHiddenInGame _array_element true)
        (Collision|SetActorEnableCollision _array_element false)))))

(event Custom|Freeroam%20Interact%20Enable
  (params (Tag :type Name))
  (bind _outactors (Actor|GetAllActorswithTag Tag))
  (for _array_element _outactors
    (if (Actor|ActorHasTag _array_element "Door")
      (Class|BPIDoor|Lock(Message) _array_element)
      (else
        (Rendering|SetActorHiddenInGame _array_element false)
        (Collision|SetActorEnableCollision _array_element true)
        (if (Actor|ActorHasTag _array_element "CharacterSidePlot")
          (Utilities|FlowControl|DoOnce false
            (:Completed
              (Utilities|FlowControl|Sequence
                (:then_0
                  (bind _outactors_2 (Actor|GetAllActorsOfClass "/Game/Blueprint/Interactables/BI_CB_Ichinose.BI_CB_Ichinose_C"))
                  (for _array_element_2 _outactors_2
                    (bind _output_get (Variables|/Game/Blueprint/BP_InteractBox.BP_InteractBox_C|SetSpawnedPlot _array_element_2 (Utilities|Array|Get(acopy) (Variables|Character|GetIchinosePlots) (Variables|Character|GetIchinoseProgress))))
                    (switch name Tag
                      (:1-7
                        (Variables|/Game/Blueprint/BP_Plot.BP_Plot_C|SetNextInteractBox _output_get "/Game/Blueprint/Interactables/BI_1-7_Discussion.BI_1-7_Discussion_C"))))))))))))
  (Utilities|FlowControl|DoOnce false) ; enters at Reset
)

(event Custom|Show%20Tutorial
  (Utilities|FlowControl|DoOnce false
    (:Completed
      (bind _returnvalue (UserInterface|CreateWidget "/Game/Blueprint/WigetBlueprints/WB_Tutorial.WB_Tutorial_C" (Game|GetPlayerController 0)))
      (UserInterface|Viewport|AddtoViewport _returnvalue 0)
      (Variables|/Script/Engine.PlayerController|SetbShowMouseCursor (Game|GetPlayerController 0) true))))

(event Custom|Check%20Special%20Event
  (switch name (Utilities|Array|Get(acopy) (Variables|Event|GetSpecialEvents) (Variables|Event|GetEventMarker))
    (:1-3
      ;[1 1 1] Special Event Check 1-3
      (bind _completed (CallFunction|1-3Check))
      (if _completed
        (bind _returnvalue (Game|SpawnActorfromClass (Variables|Chapter|GetCh1-3) (Math|Transform|MakeTransform "0, 0, 0" "0, 0, 0" "1.000000,1.000000,1.000000") "Undefined" "MultiplyWithRoot" 0 0))
        (Utilities|FlowControl|Delay 2.0)
        (Default|EnterNewDialogue (Variables|Default|GetPlayerReference) _returnvalue true "NewEnumerator0")
        (Math|Integer|IncrementInt (Variables|Event|GetEventMarker))))))

(event EventBeginPlay
  (Utilities|FlowControl|Sequence
    (:then_0
      (bind _returnvalue (Actor|GetActorOfClass "/Game/Blueprint/PlayerControl/BP_PlayerCharacter.BP_PlayerCharacter_C"))
      (bind _output_get (Variables|Default|SetPlayerReference (Variables|/Game/Blueprint/PlayerControl/BP_PlayerCharacter.BP_PlayerCharacter_C|GetAC_Player _returnvalue)))
      (bind _returnvalue_2 (Game|SpawnActorfromClass (Variables|Chapter|GetCh1-0) (Math|Transform|MakeTransform "0, 0, 0" "0, 0, 0" "1.000000,1.000000,1.000000") "Undefined" "MultiplyWithRoot" 0 0))
      (Utilities|FlowControl|Delay 0.1)
      (Default|EnterNewDialogue _output_get _returnvalue_2 true "NewEnumerator0"))
    (:then_1
      (for _array_element (Variables|Character|GetIchinosePlotClasses)
        (bind _returnvalue_3 (Game|SpawnActorfromClass _array_element (Math|Transform|MakeTransform "0, 0, 0" "0, 0, 0" "1.000000,1.000000,1.000000") "Undefined" "MultiplyWithRoot" 0 0))
        (Utilities|Array|Add (Variables|Character|GetIchinosePlots) _returnvalue_3)))))

(fn ConstructionScript)

(fn 1-3Check
  (LocalVariables|SetCheck true)
  (bind _outactors (Actor|GetAllActorsOfClasswithTag "/Game/Blueprint/BP_InteractBox.BP_InteractBox_C" "1-2"))
  (for _array_element _outactors
    (Utilities|IsValid (Variables|/Game/Blueprint/BP_InteractBox.BP_InteractBox_C|GetSpawnedPlot _array_element)
      (:Is%20Valid
        (if (not (Variables|/Game/Blueprint/BP_Plot.BP_Plot_C|GetViewed (Variables|/Game/Blueprint/BP_InteractBox.BP_InteractBox_C|GetSpawnedPlot _array_element)))
          (LocalVariables|SetCheck false)))
      (:Is%20Not%20Valid
        (LocalVariables|SetCheck false))))
  (return (LocalVariables|GetCheck)))