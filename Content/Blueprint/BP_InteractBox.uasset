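; Interactable trigger that starts a dialogue with the player, spawning its Plot actor at BeginPlay while itself starting hidden with collision off.
; Player overlap registers or clears it as the current interactable on ACPlayer and swaps the InterestMark and Mark indicators.
; Interact passes the spawned plot and camera settings to EnterNewDialogue, then calls the empty CharacterSpecial hook.
; Tick yaws InterestMark toward the player camera.
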(event EventBeginPlay
  (Utilities|FlowControl|Sequence
    (:then_0
      (Rendering|SetActorHiddenInGame true)
      (Collision|SetActorEnableCollision false)
      (Rendering|SetVisibility (Variables|Default|GetMark) false false)
      (Rendering|SetVisibility (Variables|Default|GetInterestMark) true false))
    (:then_1
      (bind _returnvalue (Game|SpawnActorfromClass (Variables|Default|GetPlot) (Math|Transform|MakeTransform "0, 0, 0" "0, 0, 0" "1.000000,1.000000,1.000000") "Undefined" "MultiplyWithRoot" 0 0))
      (Variables|Default|SetSpawnedPlot _returnvalue))))

(event Collision|EventActorBeginOverlap
  (params (OtherActor :type Actor%20Object%20Reference))
  (bind _asbp_player_character (Utilities|Casting|CastToBP_PlayerCharacter OtherActor))
  (Default|SetCurrentInteractable (Variables|/Game/Blueprint/PlayerControl/BP_PlayerCharacter.BP_PlayerCharacter_C|GetAC_Player _asbp_player_character) self)
  (Rendering|SetVisibility (Variables|Default|GetMark) true false)
  (Rendering|SetVisibility (Variables|Default|GetInterestMark) false false))

(event Collision|EventActorEndOverlap
  (params (OtherActor :type Actor%20Object%20Reference))
  (bind _asbp_player_character (Utilities|Casting|CastToBP_PlayerCharacter OtherActor))
  (Default|LeaveInteractable (Variables|/Game/Blueprint/PlayerControl/BP_PlayerCharacter.BP_PlayerCharacter_C|GetAC_Player _asbp_player_character) self)
  (Rendering|SetVisibility (Variables|Default|GetMark) false false)
  (Rendering|SetVisibility (Variables|Default|GetInterestMark) true false))

(event EventTick
  (params (DeltaSeconds :type Float%20%28single-precision%29))
  (Transformation|SetWorldRotation (Variables|Default|GetInterestMark) (Math|Rotator|MakeRotator 0.0 0.0 (.Yaw (Math|Rotator|BreakRotator (Math|Rotator|FindLookatRotation (Transformation|GetWorldLocation (Variables|Default|GetInterestMark)) (Transformation|GetWorldLocation (Variables|/Script/Engine.PlayerCameraManager|GetTransformComponent (Game|GetPlayerCameraManager 0))))))) false false))

(event EventInteract
  (params (From%20Player :type AC%20Player%20Object%20Reference))
  (Default|EnterNewDialogue From%20Player (Variables|Default|GetSpawnedPlot) (Variables|Default|GetHasSpecificCutscene) (Variables|Default|GetInteractAngle) (Transformation|GetWorldTransform (Variables|Default|GetLookat)))
  (Rendering|SetVisibility (Variables|Default|GetMark) false false)
  (CallFunction|CharacterSpecial (Variables|/Game/Blueprint/AC_Player.AC_Player_C|GetPlotManagerRef From%20Player)))

(fn ConstructionScript)

(fn CharacterSpecial
  (params (Plot%20Manager :type BP%20Plot%20Manager%20Object%20Reference)))