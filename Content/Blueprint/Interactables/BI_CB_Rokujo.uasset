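; BI_CB_Rokujo is an interactable Blueprint for Rokujo that advances this character's plot progression.
; Its CharacterSpecial function increments RokujoProgress on the passed-in PlotManager, stopping at the last index of the RokujoPlots array.
; The event graph holds only disabled default events, and the construction script just calls its parent.
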(event EventBeginPlay
  (|CallParentFunction) ; This node is disabled and will not be called.\nDrag off pins to build functionality.
)

(event Collision|EventActorBeginOverlap
  (params (OtherActor :type Actor%20Object%20Reference))
  (|CallParentFunction OtherActor) ; This node is disabled and will not be called.\nDrag off pins to build functionality.
)

(event EventTick
  (params (DeltaSeconds :type Float%20%28single-precision%29))
  (|CallParentFunction DeltaSeconds) ; This node is disabled and will not be called.\nDrag off pins to build functionality.
)

(fn ConstructionScript
  (|CallParentFunction))

(fn CharacterSpecial
  (params (Plot%20Manager :type BP%20Plot%20Manager%20Object%20Reference))
  (bind _rokujoprogress (Variables|/Game/Blueprint/BP_PlotManager.BP_PlotManager_C|GetRokujoProgress Plot%20Manager))
  (if (< _rokujoprogress (- (Utilities|Array|Length (Variables|/Game/Blueprint/BP_PlotManager.BP_PlotManager_C|GetRokujoPlots Plot%20Manager)) 1))
    (Math|Integer|IncrementInt _rokujoprogress)))