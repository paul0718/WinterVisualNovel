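; Player component that runs interaction and plot-driven dialogue, switching between free roam, interact-camera and cutscene modes.
; E messages the current interactable; EnterNewDialogue stores the plot, shows the dialogue widget and switches camera through dispatcher-style calls to the character or Level Blueprint.
; NextPage reads DataTable rows, converting bracket markup to rich-text tags and setting portrait and namebox.
; When rows run out, it restores free roam or chains another plot, handling teleports and special-event checks.
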(event Custom|Leave%20Dialogue%20Mode%20and%20Enter%20Freeroam
  (Utilities|FlowControl|Sequence
    (:then_0
      ;[1 1 1] Set Mode to Freeroam, Dismiss UI
      (CallFunction|SwitchModeto "NewEnumerator0")
      (Variables|/Script/Engine.PlayerController|SetbShowMouseCursor (Game|GetPlayerController 0) false)
      (Widget|RemovefromParent (Variables|Default|GetDialogue%20UI%20Page)))
    (:then_1
      ;[1 1 1] Reset Dialogue Markers
      (Variables|Dialogue|SetRowNum 1))))

(event Custom|Enter%20New%20Dialogue
  (params (new%20plot :type BP%20Plot%20Object%20Reference) (Has%20Specific%20Cutscene? :type Boolean) (CameraAngle :type EM_CameraAngles%20Enum :default "NewEnumerator0") (InteractAngle :type Transform))
  (Utilities|FlowControl|Sequence
    (:then_0
      ;[1 1 1] Load in plot
      (Variables|Dialogue|SetCurrentPlot new%20plot)
      (Variables|/Script/Engine.PlayerController|SetbShowMouseCursor (Game|GetPlayerController 0) true))
    (:then_1
      ;[1 1 1] Show UI, set UI
      (bind _dialogue_ui_page (Variables|Default|GetDialogue%20UI%20Page)
        (:then
          (UserInterface|Viewport|AddtoViewport _dialogue_ui_page 0))
        (:else
          (bind _returnvalue (UserInterface|CreateWidget "/Game/Blueprint/WigetBlueprints/WB_Dialogue.WB_Dialogue_C" (Game|GetPlayerController 0)))
          (bind _output_get (Variables|Default|SetDialogue%20UI%20Page _returnvalue))
          (UserInterface|Viewport|AddtoViewport _output_get 0)
          (Variables|/Game/Blueprint/WigetBlueprints/WB_Dialogue.WB_Dialogue_C|SetPlayerRefernce (Variables|Default|GetDialogue%20UI%20Page) self))))
    (:then_2
      ;[1 1 1] Switch Camera to its position
      (if Has%20Specific%20Cutscene?
        (CallFunction|SetCameratoCinemaCutscene CameraAngle)
        (else
          (CallFunction|SetCameratoInteract InteractAngle))))
    (:then_3
      (CallFunction|NextPage))))

(event EventBeginPlay
  (bind _returnvalue (Actor|GetActorOfClass "/Game/Blueprint/BP_PlotManager.BP_PlotManager_C"))
  (Variables|Ref|SetPlotManagerRef _returnvalue)
  (bind _asbp_player_character (Utilities|Casting|CastToBP_PlayerCharacter (Components|GetOwner)))
  (Variables|Ref|SetPlayerCharacterReference _asbp_player_character))

(event EventTick
  (params (DeltaSeconds :type Float%20%28single-precision%29)))

(event Input|KeyboardEvents|E
  (params (Key :type Key%20Structure :default "None"))
  (:Pressed
    (Class|BPIInteraction|Interact(Message) (Variables|Default|GetInteractable%20Item%20or%20Person) self)))

(event Custom|Next%20Page
  ;[1 1 1] Read Table
  (bind _returnvalue (Utilities|GetDataTableRow (Variables|/Game/Blueprint/BP_Plot.BP_Plot_C|GetDialogueTable (Variables|Dialogue|GetCurrentPlot)) (Utilities|String|StringToName (Utilities|String|Append "Row_" (Utilities|String|ToString(Integer) (Variables|Dialogue|GetRowNum)))))
    (:then
      (Variables|Default|SetPlotNum (.DialogueID (Utilities|Struct|BreakST_DialogueLine _returnvalue)))
      (Variables|Dialogue|SetDisplayName (.DisplayName (Utilities|Struct|BreakST_DialogueLine _returnvalue)))
      (Variables|Dialogue|SetDialogueContent (.Content (Utilities|Struct|BreakST_DialogueLine _returnvalue)))
      (Utilities|IsValid (Variables|Default|GetDialogue%20UI%20Page)
        (:Is%20Valid
          (Utilities|FlowControl|Sequence
            (:then_0
              (bind _result_rich_text (Dialogue|ProcessRawString (Variables|Dialogue|GetDialogueContent)))
              (Rendering|Components|TextRender|SetText (Variables|/Game/Blueprint/WigetBlueprints/WB_Dialogue.WB_Dialogue_C|GetMainContent (Variables|Default|GetDialogue%20UI%20Page)) _result_rich_text))
            (:then_1
              (Dialogue|SetIllustration (Variables|Dialogue|GetDisplayName))
              (CallFunction|SetNarrationHidden (Variables|Dialogue|GetDisplayName)))
            (:then_2
              (Math|Integer|IncrementInt (Variables|Dialogue|GetRowNum)))))))
    (:RowNotFound
      (Utilities|FlowControl|Sequence
        (:then_0
          (switch Utilities|FlowControl|Switch|SwitchonEM_PlotEnd (Variables|/Game/Blueprint/BP_Plot.BP_Plot_C|GetPlotEnd (Variables|Dialogue|GetCurrentPlot))
            (:NewEnumerator7
              ;[1 1 1] Leave Dialogue mode, load in tagged interactables
              (CallFunction|LeaveDialogueModeandEnterFreeroam)
              (Utilities|FlowControl|Delay (Variables|Default|GetFadeDuration))
              (Default|FreeroamInteractEnable (Variables|Ref|GetPlotManagerRef) (Variables|/Game/Blueprint/BP_Plot.BP_Plot_C|GetPlotTag (Variables|Dialogue|GetCurrentPlot)))
              (Default|ShowTutorial (Variables|Ref|GetPlotManagerRef)))
            (:NewEnumerator8
              ;[1 1 1] Leave Dialogue, load in another dialogue mode, Enter again
              (CallFunction|LeaveDialogueModeandEnterFreeroam)
              (Utilities|FlowControl|Delay (Variables|Default|GetFadeDuration))
              (bind _returnvalue_2 (Game|SpawnActorfromClass (Variables|/Game/Blueprint/BP_Plot.BP_Plot_C|GetNextInteractBox (Variables|Dialogue|GetCurrentPlot)) (Math|Transform|MakeTransform "0.000000,0.000000,30000.000000" "0, 0, 0" "1.000000,1.000000,1.000000") "Undefined" "MultiplyWithRoot" 0 0))
              (Default|Interact _returnvalue_2 self))))
        (:then_1
          ;[1 1 1] TP check
          (if (Variables|/Game/Blueprint/BP_Plot.BP_Plot_C|GetTeleport (Variables|Dialogue|GetCurrentPlot))
            (Transformation|SetActorLocation (Variables|Ref|GetPlayerCharacterReference) (Variables|/Game/Blueprint/BP_Plot.BP_Plot_C|GetTPtoLocation (Variables|Dialogue|GetCurrentPlot)) false false)))
        (:then_2
          ;[1 1 1] Special Event Check
          (Variables|/Game/Blueprint/BP_Plot.BP_Plot_C|SetViewed (Variables|Dialogue|GetCurrentPlot) true)
          (Default|CheckSpecialEvent (Variables|Ref|GetPlotManagerRef)))))))

(event Custom|Switch%20Mode%20to
  (params (To :type EM_PlayerMode%20Enum :default "NewEnumerator0"))
  (if (not (Utilities|Enum|Equal(Enum) To (Variables|State|GetMode)))
    (switch Utilities|FlowControl|Switch|SwitchonEM_PlayerMode To
      (:NewEnumerator0
        (switch Utilities|FlowControl|Switch|SwitchonEM_PlayerMode (Variables|State|GetMode)
          (:NewEnumerator8
            ;[1 1 1] Freeze to freemove
            (Default|CallPlayerCallCharactertoSwitchCameraBack)
            (Utilities|FlowControl|Delay 1.0))
          (:NewEnumerator7
            ;[1 1 1] Dialogue to Freemove
            (Default|CallPlayerCallLevelBlueprinttoEndCutscene)
            (Utilities|FlowControl|Delay (Variables|Default|GetFadeDuration))
            (CameraFades|StartCameraFade :self (Game|GetPlayerCameraManager 0) :FromAlpha 1.0 :Duration (Variables|Default|GetFadeDuration))
            (Utilities|FlowControl|Delay (Variables|Default|GetFadeDuration))))
        (Variables|State|SetMode To))
      (:NewEnumerator8
        (Variables|State|SetMode To))
      (:NewEnumerator7
        (Variables|State|SetMode To)))))

(event Custom|Set%20Camera%20to%20Interact
  (params (To%20Transform :type Transform))
  (CallFunction|SwitchModeto "NewEnumerator8")
  (Variables|Interact|SetInteractLookAtTransform To%20Transform)
  (Default|CallPlayerCallCharactertoSwitchCameratoInteract))

(event Custom|Set%20Camera%20to%20Cinema%20Cutscene
  (params (To%20angle :type EM_CameraAngles%20Enum :default "NewEnumerator0"))
  (CallFunction|SwitchModeto "NewEnumerator7")
  (Variables|State|SetCameraAngle To%20angle)
  (Default|CallPlayerCallLevelBlueprinttoPlayCutscene)
  (Default|HideAllInteractable (Variables|Ref|GetPlotManagerRef)))

(fn LeaveInteractable
  (params (From :type Actor%20Object%20Reference))
  (if (== From (Variables|Default|GetInteractable%20Item%20or%20Person))
    (Variables|Default|SetInteractable%20Item%20or%20Person 0)))

(fn SetCurrentInteractable
  (params (To :type Actor%20Object%20Reference))
  (Variables|Default|SetInteractable%20Item%20or%20Person To))

(fn SetIllustration
  (params (Selection :type EM_CharacterName%20Enum :default "NewEnumerator0"))
  (bind _characterillustration (Variables|Dialogue|GetCharacterIllustration))
  (bind _dialogue_ui_page (Variables|Default|GetDialogue%20UI%20Page))
  (bind (_value _returnvalue) (Utilities|Map|Find _characterillustration Selection))
  (bind _character (Variables|/Game/Blueprint/WigetBlueprints/WB_Dialogue.WB_Dialogue_C|GetCharacter _dialogue_ui_page))
  (if _returnvalue
    (Class|Image|SetBrush _character (Utilities|Struct|MakeSlateBrush "Image" "NoTile" "NoMirror" "(X=32.000000,Y=32.000000)" "(Left=0.000000,Top=0.000000,Right=0.000000,Bottom=0.000000)" "(SpecifiedColor=(R=1.000000,G=1.000000,B=1.000000,A=1.000000),ColorUseRule=UseColor_Specified)" "(CornerRadii=(X=0.000000,Y=0.000000,Z=0.000000,W=0.000000),Color=(SpecifiedColor=(R=0.000000,G=0.000000,B=0.000000,A=0.000000),ColorUseRule=UseColor_Specified),Width=0.000000,RoundingType=HalfHeightRadius,bUseBrushTransparency=False)" _value))
    (Widget|SetVisibility _character "Visible")
    (else
      (Widget|SetVisibility (Variables|/Game/Blueprint/WigetBlueprints/WB_Dialogue.WB_Dialogue_C|GetCharacter (Variables|Default|GetDialogue%20UI%20Page)) "Hidden"))))

(fn ProcessRawString
  (params (Raw%20String :type String))
  (return (Utilities|Text|ToText(String) (Utilities|String|Replace (Utilities|String|Replace (Utilities|String|Replace (Utilities|String|Replace Raw%20String ")-" "</>") "-(" "<H>") "]" "</>") "[" "<Bold>"))))

(fn SetNarrationHidden
  (params (Selection :type EM_CharacterName%20Enum :default "NewEnumerator0"))
  (Widget|SetVisibility (Variables|/Game/Blueprint/WigetBlueprints/WB_Dialogue.WB_Dialogue_C|GetNamebox (Variables|Default|GetDialogue%20UI%20Page)) "Visible")
  (if (Utilities|Enum|Equal(Enum) Selection "NewEnumerator7")
    (Widget|SetVisibility (Variables|/Game/Blueprint/WigetBlueprints/WB_Dialogue.WB_Dialogue_C|GetNamebox (Variables|Default|GetDialogue%20UI%20Page)) "Hidden")))